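; BP_TorchCollect is a torch collectable that the player picks up by interacting while in range.
; Sphere overlap begin and end open and close a Gate that lets the InteractwithObject event through.
; If the overlapping actor has the Player tag, it decrements LeftTorches on BP_GM_Gameplay, adds a WJ_Collectables widget to the viewport and destroys itself.
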(event OnComponentBeginOverlap(Sphere)
  (params (OverlappedComponent :type Primitive%20Component%20Object%20Reference) (OtherActor :type Actor%20Object%20Reference) (OtherComp :type Primitive%20Component%20Object%20Reference) (OtherBodyIndex :type Integer) (bFromSweep :type Boolean) (SweepResult :type Hit%20Result%20Structure%20%28by%20ref%29))
  (bind _gamemoderef (Variables|Default|GetGameModeRef))
  (Utilities|FlowControl|Gate true) ; enters at Open
)

(event OnComponentEndOverlap(Sphere)
  (params (OverlappedComponent :type Primitive%20Component%20Object%20Reference) (OtherActor :type Actor%20Object%20Reference) (OtherComp :type Primitive%20Component%20Object%20Reference) (OtherBodyIndex :type Integer))
  (bind _gamemoderef (Variables|Default|GetGameModeRef))
  (Utilities|FlowControl|Gate true) ; enters at Close
)

(event EventInteractwithObject
  (bind _gamemoderef (Variables|Default|GetGameModeRef))
  (Utilities|FlowControl|Gate true
    (:Exit
      (if (Actor|ActorHasTag (stale OnComponentBeginOverlap(Sphere) OtherActor) "Player")
        (bind _result (Math|Integer|DecrementInt (Variables|/Game/Blueprints/Core/BP_GM_Gameplay.BP_GM_Gameplay_C|GetLeftTorches _gamemoderef))
          (:%20%20
            (Variables|/Game/Blueprints/Core/BP_GM_Gameplay.BP_GM_Gameplay_C|SetLeftTorches _gamemoderef _result)
            (bind _returnvalue (UserInterface|CreateWidget "/Game/Blueprints/Widgets/WJ_Collectables.WJ_Collectables_C" (Game|GetPlayerController 0)))
            (UserInterface|Viewport|AddtoViewport _returnvalue 0)
            (Actor|DestroyActor)))))))

(event EventBeginPlay
  (bind _asbp_gm_gameplay (Utilities|Casting|CastToBP_GM_Gameplay (Game|GetGameMode)))
  (Variables|Default|SetGameModeRef _asbp_gm_gameplay))

(fn ConstructionScript)