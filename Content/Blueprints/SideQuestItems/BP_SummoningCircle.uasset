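; BP_SummoningCircle is a side-quest summoning circle that checks whether required items have been brought inside its sphere.
; On each sphere begin overlap, it recounts the overlapping actors, excluding the player character, that appear in RequiredActors.
; It prints the running count, or a summon message once the hard-coded threshold of ten is reached; no creature is actually spawned.
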(event OnComponentBeginOverlap(Sphere)
  (params (OverlappedComponent :type Primitive%20Component%20Object%20Reference) (OtherActor :type Actor%20Object%20Reference) (OtherComp :type Primitive%20Component%20Object%20Reference) (OtherBodyIndex :type Integer) (bFromSweep :type Boolean) (SweepResult :type Hit%20Result%20Structure%20%28by%20ref%29))
  (Variables|Default|SetNumberOfFoundItems 0)
  (bind _output_get (Variables|Default|SetOverlapping%20Actors (Collision|GetOverlappingActors (Variables|Default|GetSphere) 0 :!class /Script/Engine.PrimitiveComponent)))
  (Utilities|Array|RemoveItem _output_get (Game|GetPlayerCharacter 0))
  (for _array_element (Variables|Default|GetOverlapping%20Actors)
    (if (!= (Utilities|Array|FindItem (Variables|Default|GetRequiredActors) _array_element) -1)
      (Math|Integer|IncrementInt (Variables|Default|GetNumberOfFoundItems)
        (:%20%20
          (if (>= (Variables|Default|GetNumberOfFoundItems) 10)
            (Development|PrintString "SUMMON CREATURE")
            (else
              (Development|PrintString (Utilities|String|ToString(Integer) (Variables|Default|GetNumberOfFoundItems))))))))))

(event EventBeginPlay)

(event Collision|EventActorBeginOverlap
  (params (OtherActor :type Actor%20Object%20Reference)))

(event EventTick
  (params (DeltaSeconds :type Float%20%28single-precision%29)))

(fn ConstructionScript)