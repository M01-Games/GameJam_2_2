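; BP_TorchCollect is a side-quest torch actor that the player lights by interacting with it up close.
; Actor overlap events set a PlayerClose flag that gates the InteractwithObject event.
; Interacting unhides the fire component and, through a DoOnce, reports the torch to the gameplay game mode's TorchCollected, using a reference cached on BeginPlay.
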(event EventInteractwithObject
  (if (Variables|Default|GetPlayerClose)
    (Development|SetHiddeninGame (Variables|Default|GetFireButShit) false true)
    (Utilities|FlowControl|DoOnce false
      (:Completed
        (Default|TorchCollected (Variables|Default|GetGameModeRef) self)))))

(event EventBeginPlay
  (bind _asbp_gm_gameplay (Utilities|Casting|CastToBP_GM_Gameplay (Game|GetGameMode)))
  (Variables|Default|SetGameModeRef _asbp_gm_gameplay))

(event Collision|EventActorBeginOverlap
  (params (OtherActor :type Actor%20Object%20Reference))
  (Variables|Default|SetPlayerClose true))

(event Collision|EventActorEndOverlap
  (params (OtherActor :type Actor%20Object%20Reference))
  (Variables|Default|SetPlayerClose false))

(fn ConstructionScript)