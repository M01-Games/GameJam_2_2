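; BP_Trophy is a side-quest pickup that spins and bobs in place until the first-person player character overlaps it.
; Tick yaws the cube and moves the actor by BobSpeed, flipping direction only when Z exactly equals bounds set around its start height.
; On the player's first overlap, it plays a pickup sound, reports itself to BP_GM_Gameplay through TrophyCollected, then destroys itself.
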(event EventBeginPlay
  (Variables|Default|Setupper (+ (.z (Transformation|GetActorLocation)) 1e+01))
  (Variables|Default|Setlower (- (.z (Transformation|GetActorLocation)) 1e+01))
  (bind _asbp_gm_gameplay (Utilities|Casting|CastToBP_GM_Gameplay (Game|GetGameMode)))
  (Variables|Default|SetGameModeRef _asbp_gm_gameplay))

(event EventTick
  (params (DeltaSeconds :type Float%20%28single-precision%29))
  (bind _returnvalue (Transformation|GetActorLocation))
  (bind _returnvalue_2 (Transformation|GetActorLocation))
  (bind _returnvalue_3 (Transformation|GetActorLocation))
  (bind _cube (Variables|Default|GetCube))
  (bind _returnvalue_4 (Transformation|GetRelativeTransform _cube))
  (Transformation|SetRelativeRotation (Variables|Default|GetCube) (Math|Rotator|MakeRotator (.roll (.rotation _returnvalue_4)) (.pitch (.rotation _returnvalue_4)) (+ (.yaw (.rotation _returnvalue_4)) 1.0)) false false)
  (Utilities|FlowControl|Sequence
    (:then_0
      (bind _output_get (Variables|Default|Settop (== (Variables|Default|Getupper) (.z _returnvalue_3))))
      (if _output_get
        (Variables|Default|Setgo%20down true)
        (Variables|Default|Setgo%20up false)))
    (:then_1
      (bind _output_get_2 (Variables|Default|Setbottom (== (.z _returnvalue_3) (Variables|Default|Getlower))))
      (if _output_get_2
        (Variables|Default|Setgo%20up true)
        (Variables|Default|Setgo%20down false)))
    (:then_2
      (if (Variables|Default|Getgo%20up)
        (Transformation|SetActorLocation (Math|Vector|MakeVector (.x _returnvalue) (.y _returnvalue) (+ (.z _returnvalue) (/ (Variables|Default|GetBobSpeed) 1e+01))) false false)
        (elif (Variables|Default|Getgo%20down)
          (Transformation|SetActorLocation (Math|Vector|MakeVector (.x _returnvalue_2) (.y _returnvalue_2) (- (.z _returnvalue_2) (/ (Variables|Default|GetBobSpeed) 1e+01))) false false))))))

(event Collision|EventActorBeginOverlap
  (params (OtherActor :type Actor%20Object%20Reference))
  (Utilities|Casting|CastToBP_FirstPersonCharacter OtherActor)
  (Utilities|FlowControl|DoOnce false
    (:Completed
      (Audio|PlaySoundatLocation "/Game/JoeStuff/PickUpNoise.PickUpNoise" (Transformation|GetActorLocation) "0, 0, 0" 1.0 1.0 0.0 0 0 0 0)
      (Default|TrophyCollected (Variables|Default|GetGameModeRef) self)
      (Actor|DestroyActor))))

(fn ConstructionScript)