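; Spline path actor for the escort animal side quest that advances an animal position component while the player is in range.
; BeginPlay derives the spline duration from its length, giving a constant nominal speed along paths of any length.
; Tick accumulates time only while the in-range flag is set and moves the component to the spline's local transform at that time.
; Two custom events toggle the flag, so progress pauses and resumes with player proximity.
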(event Custom|PlayerIsInRange
  (Variables|Default|SetPlayerInRange true))

(event Custom|PlayerNotInRange
  (Variables|Default|SetPlayerInRange false))

(event EventBeginPlay
  (bind _spline (Variables|Default|GetSpline))
  (Variables|/Script/Engine.SplineComponent|SetDuration _spline (/ (Spline|GetSplineLength _spline) 2.5e+02)))

(event Collision|EventActorBeginOverlap
  (params (OtherActor :type Actor%20Object%20Reference)))

(event EventTick
  (params (DeltaSeconds :type Float%20%28single-precision%29))
  (if (Variables|Default|GetPlayerInRange)
    (Variables|Default|SetTimer (+ DeltaSeconds (Variables|Default|GetTimer)))
    (Transformation|SetRelativeTransform (Variables|Default|GetPositionOfAnimal) (Spline|GetTransformatTime (Variables|Default|GetSpline) (Variables|Default|GetTimer) "Local" false false) false false)))

(fn ConstructionScript)