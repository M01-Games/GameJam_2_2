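; BP_2ndCatLady is an NPC that shows a speech bubble and turns to face the player when they come close.
; On BeginPlay it stops its AI brain logic, makes the WJ_SpeechBubble widget visible and immediately adds its first dialogue text, without waiting for interaction.
; The StopLogicCollision overlaps only toggle a player-in-range flag, which Tick uses to snap the actor's rotation toward the player.
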(event OnComponentBeginOverlap(StopLogicCollision)
  (params (OverlappedComponent :type Primitive%20Component%20Object%20Reference) (OtherActor :type Actor%20Object%20Reference) (OtherComp :type Primitive%20Component%20Object%20Reference) (OtherBodyIndex :type Integer) (bFromSweep :type Boolean) (SweepResult :type Hit%20Result%20Structure%20%28by%20ref%29))
  ;[1 1 1] Stop logic and interact
  (if (Actor|ActorHasTag OtherActor "Player")
    (Variables|Default|SetPlayerInRange true)))

(event OnComponentEndOverlap(StopLogicCollision)
  (params (OverlappedComponent :type Primitive%20Component%20Object%20Reference) (OtherActor :type Actor%20Object%20Reference) (OtherComp :type Primitive%20Component%20Object%20Reference) (OtherBodyIndex :type Integer))
  ;[1 1 1] Stop logic
  (if (Actor|ActorHasTag OtherActor "Player")
    (Variables|Default|SetPlayerInRange false)))

(event Collision|EventActorBeginOverlap
  (params (OtherActor :type Actor%20Object%20Reference)))

(event EventBeginPlay
  (bind _self self)
  (bind _returnvalue (AI|GetAIController _self))
  ;[1 1 1] Reference to speech widget
  (bind _aswj_speech_bubble (Utilities|Casting|CastToWJ_SpeechBubble (UserInterface|GetWidget (Variables|Default|GetWidget))))
  (Variables|Default|SetAs%20WJ%20Speech%20Bubble _aswj_speech_bubble)
  (Utilities|IsValid _returnvalue
    (:Is%20Valid
      ;[1 1 1] Interact start
      (AI|Logic|StopLogic (Variables|/Script/AIModule.AIController|GetBrainComponent _returnvalue) ""))
    (:Is%20Not%20Valid
      _))
  (Rendering|SetVisibility (Variables|Default|GetWidget) true true)
  (if true
    (Variables|Default|SetInteracting? true)
    (bind _aswj_speech_bubble_2 (Utilities|Casting|CastToWJ_SpeechBubble (UserInterface|GetWidget (Variables|Default|GetWidget))))
    (Default|AddDialogue _aswj_speech_bubble_2 (Variables|Default|GetFirstText))))

(event EventTick
  (params (DeltaSeconds :type Float%20%28single-precision%29))
  ;[1 1 1] Focus on player
  (if (Variables|Default|GetPlayerInRange)
    (Transformation|SetActorRotation (Math|Rotator|FindLookatRotation (Transformation|GetActorLocation) (Transformation|GetActorLocation (Game|GetPlayerCharacter 0))))))

(fn ConstructionScript)