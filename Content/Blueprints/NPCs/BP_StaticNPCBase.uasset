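; Base NPC Blueprint that faces the player when nearby and offers an interaction that reveals a speech bubble.
; StopLogicCollision overlap halts the AI brain, shows an interaction prompt and clears CanMove, while Tick handles facing and removes the prompt during interaction.
; Leaving hides both widgets and restarts AI after a short delay only if InteractwithObject has set CanMove.
; AI logic is also stopped on BeginPlay.
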(event OnComponentBeginOverlap(StopLogicCollision)
  (params (OverlappedComponent :type Primitive%20Component%20Object%20Reference) (OtherActor :type Actor%20Object%20Reference) (OtherComp :type Primitive%20Component%20Object%20Reference) (OtherBodyIndex :type Integer) (bFromSweep :type Boolean) (SweepResult :type Hit%20Result%20Structure%20%28by%20ref%29))
  ;[1 1 1] Stop logic and interact
  (if (Actor|ActorHasTag OtherActor "Player")
    (Variables|Default|SetPlayerInRange true)
    (AI|Logic|StopLogic (Variables|/Script/AIModule.AIController|GetBrainComponent (AI|GetAIController self)) "")
    (Utilities|IsValid (Variables|Default|GetInteract_WJ)
      (:Is%20Valid
        _)
      (:Is%20Not%20Valid
        (bind _returnvalue (UserInterface|CreateWidget "/Game/Blueprints/Widgets/WJ_StartInteraction.WJ_StartInteraction_C" (Game|GetPlayerController 0)))))
    (bind _output_get (Variables|Default|SetInteract_WJ _returnvalue))
    (UserInterface|Viewport|AddtoViewport _output_get 0)
    (Variables|Default|SetCanMove? false)))

(event OnComponentEndOverlap(StopLogicCollision)
  (params (OverlappedComponent :type Primitive%20Component%20Object%20Reference) (OtherActor :type Actor%20Object%20Reference) (OtherComp :type Primitive%20Component%20Object%20Reference) (OtherBodyIndex :type Integer))
  ;[1 1 1] Stop logic
  (if (Actor|ActorHasTag OtherActor "Player")
    (Variables|Default|SetPlayerInRange false)
    (Rendering|SetVisibility (Variables|Default|GetWidget) false true)
    (Variables|Default|SetInteracting? false)
    (Widget|RemovefromParent (Variables|Default|GetInteract_WJ))
    (if (Variables|Default|GetCanMove?)
      (Utilities|FlowControl|Delay 1.0)
      (AI|Logic|StartLogic (Variables|/Script/AIModule.AIController|GetBrainComponent (AI|GetAIController self)))
      (Variables|Default|SetCanMove? true))))

(event EventBeginPlay
  ;[1 1 1] Reference to speech widget
  (bind _aswj_speech_bubble (Utilities|Casting|CastToWJ_SpeechBubble (UserInterface|GetWidget (Variables|Default|GetWidget))))
  (Variables|Default|SetAs%20WJ%20Speech%20Bubble _aswj_speech_bubble)
  (AI|Logic|StopLogic (Variables|/Script/AIModule.AIController|GetBrainComponent (AI|GetAIController self)) ""))

(event Collision|EventActorBeginOverlap
  (params (OtherActor :type Actor%20Object%20Reference)))

(event EventTick
  (params (DeltaSeconds :type Float%20%28single-precision%29))
  ;[1 1 1] Focus on player
  (if (Variables|Default|GetPlayerInRange)
    (Transformation|SetActorRotation (Math|Rotator|FindLookatRotation (Transformation|GetActorLocation) (Transformation|GetActorLocation (Game|GetPlayerCharacter 0))))
    (if (Variables|Default|GetInteracting?)
      (Widget|RemovefromParent (Variables|Default|GetInteract_WJ)))))

(event EventInteractwithObject
  ;[1 1 1] Interact start
  (Rendering|SetVisibility (Variables|Default|GetWidget) true true)
  (if true
    (Variables|Default|SetInteracting? true)
    (Variables|Default|SetCanMove? true)))

(fn ConstructionScript)