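; Farmer NPC that shows a speech bubble and turns to face the player when approached.
; BeginPlay loads its first dialogue line and stops its AI brain logic.
; StopLogicCollision overlaps reveal the bubble, add an interaction prompt and halt AI for the player, with delayed AI restart on exit gated by CanMove.
; Tick rotates it toward the player and removes the prompt while Interacting is set.
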(event OnComponentBeginOverlap(StopLogicCollision)
  (params (OverlappedComponent :type Primitive%20Component%20Object%20Reference) (OtherActor :type Actor%20Object%20Reference) (OtherComp :type Primitive%20Component%20Object%20Reference) (OtherBodyIndex :type Integer) (bFromSweep :type Boolean) (SweepResult :type Hit%20Result%20Structure%20%28by%20ref%29))
  (bind _self self)
  (bind _returnvalue (AI|GetAIController _self))
  (Rendering|SetVisibility (Variables|Default|GetWidget) true true)
  (if true
    (Variables|Default|SetInteracting? true)
    ;[1 1 1] Stop logic and interact
    (Variables|Default|SetCanMove? true)
    (if (Actor|ActorHasTag OtherActor "Player")
      (Variables|Default|SetPlayerInRange true)
      (Utilities|IsValid _returnvalue
        (:Is%20Valid
          (AI|Logic|StopLogic (Variables|/Script/AIModule.AIController|GetBrainComponent _returnvalue) ""))
        (:Is%20Not%20Valid
          _))
      (Utilities|IsValid (Variables|Default|GetInteract_WJ)
        (:Is%20Valid
          _)
        (:Is%20Not%20Valid
          (bind _returnvalue_2 (UserInterface|CreateWidget "/Game/Blueprints/Widgets/WJ_StartInteraction.WJ_StartInteraction_C" (Game|GetPlayerController 0)))))
      (bind _output_get (Variables|Default|SetInteract_WJ _returnvalue_2))
      (UserInterface|Viewport|AddtoViewport _output_get 0)
      (Variables|Default|SetCanMove? false))))

(event OnComponentEndOverlap(StopLogicCollision)
  (params (OverlappedComponent :type Primitive%20Component%20Object%20Reference) (OtherActor :type Actor%20Object%20Reference) (OtherComp :type Primitive%20Component%20Object%20Reference) (OtherBodyIndex :type Integer))
  (bind _self self)
  (bind _returnvalue (AI|GetAIController _self))
  ;[1 1 1] Stop logic
  (if (Actor|ActorHasTag OtherActor "Player")
    (Variables|Default|SetPlayerInRange false)
    (Rendering|SetVisibility (Variables|Default|GetWidget) false true)
    (Variables|Default|SetInteracting? false)
    (Widget|RemovefromParent (Variables|Default|GetInteract_WJ))
    (if (Variables|Default|GetCanMove?)
      (Utilities|FlowControl|Delay 1.0)
      (Utilities|IsValid _returnvalue
        (:Is%20Valid
          (AI|Logic|StartLogic (Variables|/Script/AIModule.AIController|GetBrainComponent _returnvalue)))
        (:Is%20Not%20Valid
          _))
      (Variables|Default|SetCanMove? true))))

(event EventBeginPlay
  (bind _self self)
  (bind _returnvalue (AI|GetAIController _self))
  ;[1 1 1] Reference to speech widget
  (bind _aswj_speech_bubble (Utilities|Casting|CastToWJ_SpeechBubble (UserInterface|GetWidget (Variables|Default|GetWidget))))
  (Variables|Default|SetAs%20WJ%20Speech%20Bubble _aswj_speech_bubble)
  (Utilities|IsValid _returnvalue
    (:Is%20Valid
      (AI|Logic|StopLogic (Variables|/Script/AIModule.AIController|GetBrainComponent _returnvalue) ""))
    (:Is%20Not%20Valid
      _))
  (bind _aswj_speech_bubble_2 (Utilities|Casting|CastToWJ_SpeechBubble (UserInterface|GetWidget (Variables|Default|GetWidget))))
  (Default|AddDialogue _aswj_speech_bubble_2 (Variables|Default|GetFirstText)))

(event Collision|EventActorBeginOverlap
  (params (OtherActor :type Actor%20Object%20Reference)))

(event EventTick
  (params (DeltaSeconds :type Float%20%28single-precision%29))
  ;[1 1 1] Focus on player
  (if (Variables|Default|GetPlayerInRange)
    (Transformation|SetActorRotation (Math|Rotator|FindLookatRotation (Transformation|GetActorLocation) (Transformation|GetActorLocation (Game|GetPlayerCharacter 0))))
    (if (Variables|Default|GetInteracting?)
      (Widget|RemovefromParent (Variables|Default|GetInteract_WJ)))))

(fn ConstructionScript)