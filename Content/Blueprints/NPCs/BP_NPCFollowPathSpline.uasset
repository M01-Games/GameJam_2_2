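; NPC path spline actor that builds two side lanes along its spline and locates the path point nearest an AI position.
; BeginPlay samples the spline at fixed intervals into left and right offset point arrays.
; Getclosestpointtoai keeps the nearer side per sample, picks the last one closer than its predecessor, and stores its index.
; Persistent sphere traces and prints expose debug results; furthest-left and lowest-point loops are unwired.
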(event Custom|Get%20closest%20point%20to%20ai
  (params (AI%20Position :type Vector))
  (bind (_x _y) (Class|KismetMathLibrary|BreakVector3f AI%20Position))
  (bind _closest_points (Variables|Default|GetClosest%20Points))
  (bind _closest_points_2 (Variables|Default|GetClosest%20Points))
  (for (_array_element _array_index) (Variables|Default|GetLeftSidePoints)
    (Math|Float|CompareFloat (Math|Vector|Distance2D(Vector) (Math|Vector2D|MakeVector2D (.X (Class|KismetMathLibrary|BreakVector3f _array_element)) (.Y (Class|KismetMathLibrary|BreakVector3f _array_element))) (Math|Vector2D|MakeVector2D _x _y)) (Math|Vector|Distance2D(Vector) (Math|Vector2D|MakeVector2D (.X (Class|KismetMathLibrary|BreakVector3f (Utilities|Array|Get(acopy) (Variables|Default|GetRightSidePoints) _array_index))) (.Y (Class|KismetMathLibrary|BreakVector3f (Utilities|Array|Get(acopy) (Variables|Default|GetRightSidePoints) _array_index)))) (Math|Vector2D|MakeVector2D _x _y))
      (:>
        (Utilities|Array|Add _closest_points (Utilities|Array|Get(acopy) (Variables|Default|GetRightSidePoints) _array_index)))
      (:<
        (Utilities|Array|Add _closest_points _array_element))))
  (for _array_element_2 (Variables|Default|GetClosest%20Points)
    (Collision|SphereTraceByChannel _array_element_2 _array_element_2 1e+01 "TraceTypeQuery1" false 0 "Persistent"))
  (for (_array_element_3 _array_index_2) _closest_points_2
    (if (not (== _array_index_2 0))
      (Development|PrintString (Utilities|String|ToString(Float) (Math|Vector|Distance2D(Vector) (Math|Vector2D|MakeVector2D (.X (Class|KismetMathLibrary|BreakVector3f _array_element_3)) (.Y (Class|KismetMathLibrary|BreakVector3f _array_element_3))) (Math|Vector2D|MakeVector2D _x _y))))
      (if (< (Math|Vector|Distance2D(Vector) (Math|Vector2D|MakeVector2D (.X (Class|KismetMathLibrary|BreakVector3f _array_element_3)) (.Y (Class|KismetMathLibrary|BreakVector3f _array_element_3))) (Math|Vector2D|MakeVector2D _x _y)) (Math|Vector|Distance2D(Vector) (Math|Vector2D|MakeVector2D (.X (Class|KismetMathLibrary|BreakVector3f (Utilities|Array|Get(acopy) _closest_points_2 (- _array_index_2 1)))) (.Y (Class|KismetMathLibrary|BreakVector3f (Utilities|Array|Get(acopy) _closest_points_2 (- _array_index_2 1))))) (Math|Vector2D|MakeVector2D _x _y)))
        (Variables|Default|SetAbsoluteClosest _array_element_3))))
  (Development|PrintString (Utilities|String|ToString(Float) (Math|Vector|Distance2D(Vector) (Math|Vector2D|MakeVector2D (.x (Variables|Default|GetAbsoluteClosest)) (.y (Variables|Default|GetAbsoluteClosest))) (Math|Vector2D|MakeVector2D _x _y))))
  (if (== (Utilities|Array|FindItem (Variables|Default|GetLeftSidePoints) (Variables|Default|GetAbsoluteClosest)) -1)
    (Variables|Default|SetClosestPointIndex (Utilities|Array|FindItem (Variables|Default|GetRightSidePoints) (Variables|Default|GetAbsoluteClosest)))
    (else
      (Variables|Default|SetClosestPointIndex (Utilities|Array|FindItem (Variables|Default|GetLeftSidePoints) (Variables|Default|GetAbsoluteClosest)))))
  (Collision|SphereTraceByChannel (Utilities|Array|Get(acopy) (Variables|Default|GetLeftSidePoints) (Variables|Default|GetClosestPointIndex)) (Utilities|Array|Get(acopy) (Variables|Default|GetRightSidePoints) (Variables|Default|GetClosestPointIndex)) 1e+01 "TraceTypeQuery1" false 0 "Persistent"))

(event Collision|EventActorBeginOverlap
  (params (OtherActor :type Actor%20Object%20Reference)))

(event EventTick
  (params (DeltaSeconds :type Float%20%28single-precision%29)))

(event EventBeginPlay
  (bind _spline (Variables|Default|GetSpline))
  (Spline|SetClosedLoop (Variables|Default|GetSpline) (Variables|Default|GetLoopSpline) true)
  (for _index (range 0 (Math|Float|Round (/ (Spline|GetSplineLength _spline) 2e+01)))
    (Utilities|Array|Add (Variables|Default|GetLeftSidePoints) (- (Spline|GetLocationatDistanceAlongSpline _spline (* _index 2e+01) "World") (* (Class|SplineComponent|GetRightVectoratDistanceAlongSpline _spline (* _index 2e+01) "World") 1e+02)))
    (Utilities|Array|Add (Variables|Default|GetRightSidePoints) (- (Spline|GetLocationatDistanceAlongSpline _spline (* _index 2e+01) "World") (* (Class|SplineComponent|GetRightVectoratDistanceAlongSpline _spline (* _index 2e+01) "World") -1e+02)))
    (Collision|SphereTraceByChannel (- (Spline|GetLocationatDistanceAlongSpline _spline (* _index 2e+01) "World") (* (Class|SplineComponent|GetRightVectoratDistanceAlongSpline _spline (* _index 2e+01) "World") 1e+02)) (- (Spline|GetLocationatDistanceAlongSpline _spline (* _index 2e+01) "World") (* (Class|SplineComponent|GetRightVectoratDistanceAlongSpline _spline (* _index 2e+01) "World") 1e+02)) 1e+01 "TraceTypeQuery1" false 0 "None")
    (Collision|SphereTraceByChannel (- (Spline|GetLocationatDistanceAlongSpline _spline (* _index 2e+01) "World") (* (Class|SplineComponent|GetRightVectoratDistanceAlongSpline _spline (* _index 2e+01) "World") -1e+02)) (- (Spline|GetLocationatDistanceAlongSpline _spline (* _index 2e+01) "World") (* (Class|SplineComponent|GetRightVectoratDistanceAlongSpline _spline (* _index 2e+01) "World") -1e+02)) 1e+01 "TraceTypeQuery1" false 0 "None")))

(fn ConstructionScript)