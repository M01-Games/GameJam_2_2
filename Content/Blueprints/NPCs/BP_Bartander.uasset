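; BP_Bartander is a bartender NPC that shows an opening line of dialogue in a speech bubble.
; On BeginPlay it runs the parent logic, then casts its widget component's widget to WJ_SpeechBubble and adds FirstText as dialogue.
; The overlap and tick events are disabled, and the construction script only calls the parent.
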(event EventBeginPlay
  (|CallParentFunction)
  (bind _aswj_speech_bubble (Utilities|Casting|CastToWJ_SpeechBubble (UserInterface|GetWidget (Variables|Default|GetWidget))))
  (Default|AddDialogue _aswj_speech_bubble (Variables|Default|GetFirstText)))

(event Collision|EventActorBeginOverlap
  (params (OtherActor :type Actor%20Object%20Reference))
  (|CallParentFunction OtherActor) ; This node is disabled and will not be called.\nDrag off pins to build functionality.
)

(event EventTick
  (params (DeltaSeconds :type Float%20%28single-precision%29))
  (|CallParentFunction DeltaSeconds) ; This node is disabled and will not be called.\nDrag off pins to build functionality.
)

(fn ConstructionScript
  (|CallParentFunction))