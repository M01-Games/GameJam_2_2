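; BP_RandomPeople is an NPC Blueprint that shows random lines of dialogue in a speech bubble.
; On begin play it adds a random FirstText line to the WJ_SpeechBubble held by its Widget.
; When CallEnvironmentalInteract fires, it makes the Widget visible and adds a random ReactionText line to the same bubble.
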(event EventBeginPlay
  (bind _firsttext (Variables|Default|GetFirstText))
  (|CallParentFunction)
  (bind _aswj_speech_bubble (Utilities|Casting|CastToWJ_SpeechBubble (UserInterface|GetWidget (Variables|Default|GetWidget))))
  (Default|AddDialogue _aswj_speech_bubble (Utilities|Array|Get(acopy) _firsttext (Math|Random|RandomIntegerinRange 0 (- (Utilities|Array|Length _firsttext) 1)))))

(event EventCallEnvironmentalInteract
  (bind _widget (Variables|Default|GetWidget))
  (bind _reactiontext (Variables|Default|GetReactionText))
  (Rendering|SetVisibility _widget true true)
  (bind _aswj_speech_bubble (Utilities|Casting|CastToWJ_SpeechBubble (UserInterface|GetWidget _widget)))
  (Default|AddDialogue _aswj_speech_bubble (Utilities|Array|Get(acopy) _reactiontext (Math|Random|RandomIntegerinRange 0 (- (Utilities|Array|Length _reactiontext) 1)))))

(fn ConstructionScript
  (|CallParentFunction))