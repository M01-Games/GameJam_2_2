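; Cat quest tree actor that can be knocked down once it has been made breakable.
; MakeTreeBreakable sets the Breakable flag, which gates the Box overlap check for a Destructive_Objects_BP actor.
; The first valid overlap calls TreeFalling on the cached BP_GM_Gameplay game mode, then destroys the tree.
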(event OnComponentBeginOverlap(Box)
  (params (OverlappedComponent :type Primitive%20Component%20Object%20Reference) (OtherActor :type Actor%20Object%20Reference) (OtherComp :type Primitive%20Component%20Object%20Reference) (OtherBodyIndex :type Integer) (bFromSweep :type Boolean) (SweepResult :type Hit%20Result%20Structure%20%28by%20ref%29))
  (if (Variables|Default|GetBreakable)
    (Utilities|Casting|CastToDestructive_Objects_BP OtherActor)
    (Utilities|FlowControl|DoOnce false
      (:Completed
        (Default|TreeFalling (Variables|Default|GetGameModeRef))
        (Actor|DestroyActor)))))

(event Custom|MakeTreeBreakable
  (Variables|Default|SetBreakable true))

(event EventBeginPlay
  (bind _asbp_gm_gameplay (Utilities|Casting|CastToBP_GM_Gameplay (Game|GetGameMode)))
  (Variables|Default|SetGameModeRef _asbp_gm_gameplay))

(event Collision|EventActorBeginOverlap
  (params (OtherActor :type Actor%20Object%20Reference)))

(event EventTick
  (params (DeltaSeconds :type Float%20%28single-precision%29)))

(fn ConstructionScript)