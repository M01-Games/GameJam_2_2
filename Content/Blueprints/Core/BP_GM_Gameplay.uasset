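; Gameplay game mode that drives a linear quest chain: bar drink, cat in a tree, farmer's hay bales, then home to bed.
; BeginPlay caches level actors and spawn markers, counts torch and trophy collectibles, and creates the task widget.
; Custom events advance each stage, spawning NPCs and props and updating task dialogue.
; Clearing all hay enables home detection; sleeping only prints a win message, with the end cutscene unimplemented.
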(event Custom|Activate%20BarTask
  ;[1 1 1] Trigger for bar Task
  ;;[1 1 1] Add ui for the task on screen
  (Default|AddDialogue (Variables|Default|GettaskRef) "Good Morning! Let's go  
get a drink at the bar. 
"))

(event Custom|SpawnBeerMug
  ;[1 1 1] Trigger for bar Task
  (Game|SpawnActorfromClass "/Game/Blueprints/MainQuestItems/TavernQuestItems/BP_BeerMug.BP_BeerMug_C" (Math|Transform|MakeTransform (Variables|Default|GetBeerSpwanLocation) "0, 0, 0" "1.000000,1.000000,1.000000") "Undefined" "MultiplyWithRoot" 0 0))

(event Custom|Spoken%20to%20cat%20lady
  ;[1 1 1] Trigger for bar Task
  (Default|AddDialogue (Variables|Default|GettaskRef) "Help the cat out 
of the tree near 
the farm."))

(event Custom|SleptInBed
  ;[1 1 1] Trigger End cutscene and finish game
  ;;[1 1 1] Play end cutscene here
  (Development|PrintString "YOU WIN"))

(event Custom|ActivateCatTask
  ;[1 1 1] Trigger for mission 1 cat task
  ;;[1 1 1] Spawn Cat perons NPC here
  (bind _returnvalue (Game|SpawnActorfromClass "/Game/Blueprints/NPCs/BP_1stCatLady.BP_1stCatLady_C" (Transformation|GetActorTransform (Variables|Default|GetCatLadySpawn1)) "Undefined" "MultiplyWithRoot" 0 0))
  (Variables|Default|SetCatLady1Ref _returnvalue)
  (Default|MakeTreeBreakable (Variables|Default|GetTreeRef)))

(event Custom|BeerMugPickedUp
  ;[1 1 1] Trigger for bar Task
  (Default|GrowHands (Variables|Default|GetCharacterRef))
  (CallFunction|ActivateCatTask)
  ;;[1 1 1] Remove Beer Objective from screen
  (Default|AddDialogue (Variables|Default|GettaskRef) "Talk to the lady  
inside the bar. 
She needs help."))

(event Custom|TreeFalling
  (bind _characterref (Variables|Default|GetCharacterRef))
  ;[1 1 1] Trigger for bar Task
  ;[1 1 1] Trigger for mission 1 cat task
  (Default|BreakFence (Variables|Default|GetFenceRef))
  (Actor|DestroyActor (Variables|Default|GetCatLady1Ref))
  (bind _returnvalue (Game|SpawnActorfromClass "/Game/Blueprints/MainQuestItems/CatQuest/BP_Cat.BP_Cat_C" (Transformation|GetActorTransform (Variables|Default|GetCatSpawnPoint)) "Undefined" "MultiplyWithRoot" 0 0))
  (Pawn|SpawnDefaultController _returnvalue)
  (bind _returnvalue_2 (Game|SpawnActorfromClass "/Game/Blueprints/NPCs/BP_2ndCatLady.BP_2ndCatLady_C" (Transformation|GetActorTransform (Variables|Default|GetCatLadySpawn2)) "Undefined" "MultiplyWithRoot" 0 0))
  (Variables|Default|SetCatLady2 _returnvalue_2)
  ;;[1 1 1] Spawn Farmer NPC here
  (bind _returnvalue_3 (Game|SpawnActorfromClass "/Game/Blueprints/NPCs/BP_1stFarmer.BP_1stFarmer_C" (Math|Transform|MakeTransform (+ (* (Math|Vector|GetForwardVector (Variables|/Game/FirstPerson/Blueprints/BP_FirstPersonCharacter.BP_FirstPersonCharacter_C|GetFirstPersonCamera _characterref)) 2e+02) (Transformation|GetActorLocation _characterref)) "0, 0, 0" "1.000000,1.000000,1.000000") "Undefined" "MultiplyWithRoot" 0 0))
  (Variables|Default|SetFarmer1Ref _returnvalue_3)
  (Utilities|FlowControl|Delay 4.0)
  (Default|AddDialogue (Variables|Default|GettaskRef) "Help the farmer 
move 5 hay.")
  (CallFunction|ActivateFarmerTask))

(event Custom|ActivateFarmerTask
  ;[1 1 1] Trigger for Mission 2 Farmer Task
  (for _array_element (Variables|Default|GetHaySpawnLocations)
    (bind _returnvalue (Game|SpawnActorfromClass "/Game/Blueprints/MainQuestItems/FarmerQuest/BP_HayBale.BP_HayBale_C" (Transformation|GetActorTransform _array_element) "Undefined" "MultiplyWithRoot" 0 0))
    (Utilities|Array|Add (Variables|Default|GetAllHayBales) _returnvalue)))

(event Custom|HayBaleDestroyed
  (params (Hay%20Bale%20Ref :type BP%20Hay%20Bale%20Object%20Reference))
  ;[1 1 1] Trigger for Mission 2 Farmer Task
  (Utilities|Array|RemoveItem (Variables|Default|GetAllHayBales) Hay%20Bale%20Ref)
  (Variables|Default|SetNumOfHayBalesLeft (- (Utilities|Array|Length (Variables|Default|GetHaySpawnLocations)) (Utilities|Array|Length (Variables|Default|GetAllHayBales))))
  (Utilities|IsValid (Utilities|Array|Get(acopy) (Variables|Default|GetAllHayBales))
    (:Is%20Not%20Valid
      (CallFunction|SpawnFarmerforSecondTime)
      (Default|AddDialogue (Variables|Default|GettaskRef) "Go back home and rest."))))

(event Custom|SpawnFarmerForSecondTime
  (bind _characterref (Variables|Default|GetCharacterRef))
  ;[1 1 1] Trigger for Mission 2 Farmer Task
  (Actor|DestroyActor (Variables|Default|GetFarmer1Ref))
  (Game|SpawnActorfromClass "/Game/Blueprints/NPCs/BP_2ndFarmer.BP_2ndFarmer_C" (Math|Transform|MakeTransform (+ (* (Math|Vector|GetForwardVector (Variables|/Game/FirstPerson/Blueprints/BP_FirstPersonCharacter.BP_FirstPersonCharacter_C|GetFirstPersonCamera _characterref)) 2e+02) (Transformation|GetActorLocation _characterref)) "0, 0, 0" "1.000000,1.000000,1.000000") "Undefined" "MultiplyWithRoot" 0 0)
  (Variables|/Game/Blueprints/MainQuestItems/GoBackHomeTask/BP_AtHomeDetection.BP_AtHomeDetection_C|SetCanBeActivated (Variables|Default|GetHomeDetectionRef) true))

(event EventTick
  (params (DeltaSeconds :type Float%20%28single-precision%29)))

(event EventBeginPlay
  ;[1 1 1] Begin play Fuctnions
  (bind _spawnlocation (CallFunction|GetBeerSpawnLocation))
  (Variables|Default|SetBeerSpwanLocation _spawnlocation)
  (bind _asbp_first_person_character (Utilities|Casting|CastToBP_FirstPersonCharacter (Game|GetPlayerCharacter 0)))
  (Variables|Default|SetCharacterRef _asbp_first_person_character)
  (bind _returnvalue (Actor|GetActorOfClass "/Game/Blueprints/MainQuestItems/CatQuest/BP_TreeWithCatIn.BP_TreeWithCatIn_C"))
  (Variables|Default|SetTreeRef _returnvalue)
  (bind _returnvalue_2 (Actor|GetActorOfClass "/Game/Blueprints/MainQuestItems/CatQuest/BP_Fence.BP_Fence_C"))
  (Variables|Default|SetFenceRef _returnvalue_2)
  (bind _outactors (Actor|GetAllActorsOfClass "/Game/Blueprints/MainQuestItems/FarmerQuest/BP_HaySpawnLocations.BP_HaySpawnLocations_C"))
  (Variables|Default|SetHaySpawnLocations _outactors)
  (bind _outactors_2 (Actor|GetAllActorsOfClass "/Game/Blueprints/SideQuestItems/Collectables/BP_TorchCollect.BP_TorchCollect_C"))
  (Variables|Default|SetAllTorchCollectables _outactors_2)
  (bind _outactors_3 (Actor|GetAllActorsOfClass "/Game/Blueprints/SideQuestItems/Collectables/BP_Trophy.BP_Trophy_C"))
  (Variables|Default|SetAllTrophyCollectables _outactors_3)
  (bind _returnvalue_3 (Actor|GetActorOfClass "/Game/Blueprints/MainQuestItems/GoBackHomeTask/BP_AtHomeDetection.BP_AtHomeDetection_C"))
  (Variables|Default|SetHomeDetectionRef _returnvalue_3)
  (bind _returnvalue_4 (Actor|GetActorOfClass "/Game/Blueprints/MainQuestItems/CatQuest/BP_CatLadySpawnPoint1.BP_CatLadySpawnPoint1_C"))
  (Variables|Default|SetCatLadySpawn1 _returnvalue_4)
  (bind _returnvalue_5 (Actor|GetActorOfClass "/Game/Blueprints/MainQuestItems/CatQuest/BP_CatLadySpawnPoint2.BP_CatLadySpawnPoint2_C"))
  (Variables|Default|SetCatLadySpawn2 _returnvalue_5)
  (bind _returnvalue_6 (UserInterface|CreateWidget "/Game/Blueprints/Widgets/WJ_TaskProgressMenu.WJ_TaskProgressMenu_C" (Game|GetPlayerController 0)))
  (bind _output_get (Variables|Default|SettaskRef _returnvalue_6))
  (UserInterface|Viewport|AddtoViewport _output_get 0)
  (CallFunction|ActivateBarTask)
  (bind _outactors_4 (Actor|GetAllActorsOfClass "/Game/Blueprints/SideQuestItems/Collectables/BP_TorchCollect.BP_TorchCollect_C"))
  (bind _output_get_2 (Variables|Default|SetLeftTorches (Utilities|Array|Length _outactors_4)))
  (Variables|Default|SetTotalTorches _output_get_2)
  (bind _outactors_5 (Actor|GetAllActorsOfClass "/Game/Blueprints/SideQuestItems/Collectables/BP_Trophy.BP_Trophy_C"))
  (bind _output_get_3 (Variables|Default|SetLeftTrophies (Utilities|Array|Length _outactors_5)))
  (Variables|Default|SetTotalTrophies _output_get_3)
  (bind _returnvalue_7 (Actor|GetActorOfClass "/Game/Blueprints/MainQuestItems/CatQuest/BP_CatSpawnPoint.BP_CatSpawnPoint_C"))
  (Variables|Default|SetCatSpawnPoint _returnvalue_7))

(fn ConstructionScript)

(fn GetBeerSpawnLocation
  (bind _returnvalue (Actor|GetActorOfClass "/Game/Blueprints/MainQuestItems/TavernQuestItems/BP_BeerSpwanLocation.BP_BeerSpwanLocation_C"))
  (return (Transformation|GetActorLocation _returnvalue)))