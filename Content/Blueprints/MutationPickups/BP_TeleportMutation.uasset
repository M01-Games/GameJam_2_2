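; BP_TeleportMutation is a pickup actor that grants the first-person character the teleport mutation.
; BeginPlay caches player 0's BP_FirstPersonCharacter, and any Box overlap calls PickedupTeleportMut on it without checking which actor entered.
; A HasBeenTriggered flag blocks repeat triggers until ReativateCollision clears it after a 30-second delay, making the pickup reusable without toggling collision or visibility.
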(event OnComponentBeginOverlap(Box)
  (params (OverlappedComponent :type Primitive%20Component%20Object%20Reference) (OtherActor :type Actor%20Object%20Reference) (OtherComp :type Primitive%20Component%20Object%20Reference) (OtherBodyIndex :type Integer) (bFromSweep :type Boolean) (SweepResult :type Hit%20Result%20Structure%20%28by%20ref%29))
  (if (not (Variables|Default|GetHasBeenTriggered))
    (Variables|Default|SetHasBeenTriggered true)
    (CallFunction|ReativateCollision)
    (Default|PickedupTeleportMut (Variables|Default|GetPlayerRef))))

(event Custom|ReativateCollision
  (Utilities|FlowControl|Delay 3e+01)
  (Variables|Default|SetHasBeenTriggered false))

(event EventBeginPlay
  (bind _asbp_first_person_character (Utilities|Casting|CastToBP_FirstPersonCharacter (Game|GetPlayerCharacter 0)))
  (Variables|Default|SetPlayerRef _asbp_first_person_character))

(event Collision|EventActorBeginOverlap
  (params (OtherActor :type Actor%20Object%20Reference)))

(event EventTick
  (params (DeltaSeconds :type Float%20%28single-precision%29)))

(fn ConstructionScript)