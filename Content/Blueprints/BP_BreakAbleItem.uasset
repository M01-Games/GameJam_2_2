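; Breakable prop that shatters when a Destructive_Objects_BP overlaps its collision and alerts nearby NPCs.
; Mesh and material are applied in the construction script, and the particle asset is assigned at BeginPlay.
; A detection volume tracks BP_NPCBase actors in range.
; On the first hit it plays effect and sound, hides the mesh, calls each tracked NPC's environmental interact, then destroys itself after a short delay.
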(event OnComponentBeginOverlap(Collision)
  (params (OverlappedComponent :type Primitive%20Component%20Object%20Reference) (OtherActor :type Actor%20Object%20Reference) (OtherComp :type Primitive%20Component%20Object%20Reference) (OtherBodyIndex :type Integer) (bFromSweep :type Boolean) (SweepResult :type Hit%20Result%20Structure%20%28by%20ref%29))
  (bind _niagara (Variables|Default|GetNiagara))
  (bind _staticmesh (Variables|Default|GetStaticMesh))
  (Utilities|Casting|CastToDestructive_Objects_BP OtherActor)
  (Utilities|FlowControl|DoOnce false
    (:Completed
      (Niagara|ResetSystem _niagara)
      (Development|SetHiddeninGame _niagara false false)
      (Audio|PlaySoundatLocation (Variables|Default|GetSoundToPlay) (Transformation|GetActorLocation) "0, 0, 0" 1.0 1.0 0.0 0 0 0 0)
      (Development|SetHiddeninGame _staticmesh true false)
      (Collision|SetCollisionEnabled _staticmesh "NoCollision")
      (for _array_element (Variables|Default|GetArrayOfNpcsInRange)
        (Default|CallEnvironmentalInteract _array_element))
      (Utilities|FlowControl|Delay 2.0)
      (Actor|DestroyActor))))

(event OnComponentBeginOverlap(DetectNPC)
  (params (OverlappedComponent :type Primitive%20Component%20Object%20Reference) (OtherActor :type Actor%20Object%20Reference) (OtherComp :type Primitive%20Component%20Object%20Reference) (OtherBodyIndex :type Integer) (bFromSweep :type Boolean) (SweepResult :type Hit%20Result%20Structure%20%28by%20ref%29))
  (bind _asbp_npcbase (Utilities|Casting|CastToBP_NPCBase OtherActor))
  (Utilities|Array|Add (Variables|Default|GetArrayOfNpcsInRange) _asbp_npcbase))

(event OnComponentEndOverlap(DetectNPC)
  (params (OverlappedComponent :type Primitive%20Component%20Object%20Reference) (OtherActor :type Actor%20Object%20Reference) (OtherComp :type Primitive%20Component%20Object%20Reference) (OtherBodyIndex :type Integer))
  (bind _asbp_npcbase (Utilities|Casting|CastToBP_NPCBase OtherActor))
  (Utilities|Array|RemoveItem (Variables|Default|GetArrayOfNpcsInRange) _asbp_npcbase))

(event EventBeginPlay
  (Class|NiagaraComponent|SetAsset (Variables|Default|GetNiagara) (Variables|Default|GetParticleToSpawn) true))

(event Collision|EventActorBeginOverlap
  (params (OtherActor :type Actor%20Object%20Reference)))

(event EventTick
  (params (DeltaSeconds :type Float%20%28single-precision%29)))

(fn ConstructionScript
  (bind _staticmesh (Variables|Default|GetStaticMesh))
  (Components|StaticMesh|SetStaticMesh _staticmesh (Variables|Default|GetMeshToUse))
  (Rendering|Material|SetMaterial _staticmesh 0 (Variables|Default|GetMaterialToUse)))